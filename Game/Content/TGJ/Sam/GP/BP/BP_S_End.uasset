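; End-of-game interaction actor that plays the chapter 3 ending sequence, then shows the end screen.
; While BP_3rdPers overlaps its Sphere, its Interaction event is bound to the GI_TGJ_Main start-interaction event, and unbound on exit.
; Interaction changes the game instance's GameMode state, plays S_Chap3_End, waits for a delay taken from the sequence's end time, then adds W_End to the viewport.
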(event `self.ReceiveBeginPlay`
  (bind _asgi_tgj_main (cast `/Game/TGJ/Sam/GP/3rdPers/BP/GI_TGJ_Main` (`GameplayStatics.GetGameInstance`)))
  (set `self.As GI TGJ Main` _asgi_tgj_main))

(event `self.Sphere.OnComponentEndOverlap`
  (params (OverlappedComponent :type "PrimitiveComponent Object Reference") (OtherActor :type "Actor Object Reference") (OtherComp :type "PrimitiveComponent Object Reference") (OtherBodyIndex :type Integer))
  (bind _asbp_3rd_pers (cast `/Game/TGJ/Sam/GP/3rdPers/BP/BP_3rdPers` OtherActor))
  (set `self.As BP Third Person Character` _asbp_3rd_pers)
  (remove `/Game/TGJ/Sam/GP/3rdPers/BP/GI_TGJ_Main.StartInteraction` (`self.As GI TGJ Main`) (delegate `Interaction`)))

(event `self.Sphere.OnComponentBeginOverlap`
  (params (OverlappedComponent :type "PrimitiveComponent Object Reference") (OtherActor :type "Actor Object Reference") (OtherComp :type "PrimitiveComponent Object Reference") (OtherBodyIndex :type Integer) (bFromSweep :type Boolean) (SweepResult :type "HitResult Structure (by ref)"))
  (bind _asbp_3rd_pers (cast `/Game/TGJ/Sam/GP/3rdPers/BP/BP_3rdPers` OtherActor))
  (set `self.As BP Third Person Character` _asbp_3rd_pers)
  (add `/Game/TGJ/Sam/GP/3rdPers/BP/GI_TGJ_Main.StartInteraction` (`self.As GI TGJ Main`) (delegate `Interaction`)))

(event `Interaction`
  (set `/Game/TGJ/Sam/GP/3rdPers/BP/GI_TGJ_Main.GameMode` "NewEnumerator5" (`self.As GI TGJ Main`))
  (bind (_outactor _returnvalue) (`LevelSequencePlayer.CreateLevelSequencePlayer` "/Game/TGJ/Sam/C/S_Chap3_End.S_Chap3_End"))
  (`MovieSceneSequencePlayer.Play` (`LevelSequenceActor.SequencePlayer` _outactor))
  (`KismetSystemLibrary.Delay` (`TimeManagementBlueprintLibrary.Conv_QualifiedFrameTimeToSeconds` (`MovieSceneSequencePlayer.GetEndTime` _returnvalue)))
  (bind _returnvalue_2 (`|CreateWidget` "/Game/TGJ/Oz/UMG/W/W_End.W_End_C"))
  (`UserWidget.AddToViewport` _returnvalue_2 0))

(fn `UserConstructionScript`)