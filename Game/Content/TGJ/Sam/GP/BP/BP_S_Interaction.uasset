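; Interactable actor that plays a one-time, red/blue color-themed response when the player interacts within range.
; Sphere overlaps with BP_3rdPers bind and unbind its Interaction event on the game instance's start-interaction dispatch.
; Interaction either hands itself to the game instance's graduation interaction or shows an emote widget, optionally preceded by Niagara and material FX.
; Emote animation follows the character's or actor's Blue flag, with single or paired textures.
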(event `self.ReceiveBeginPlay`
  (bind _asgi_tgj_main (cast `/Game/TGJ/Sam/GP/3rdPers/BP/GI_TGJ_Main` (`GameplayStatics.GetGameInstance`)))
  (set `self.As GI TGJ Main` _asgi_tgj_main))

(event `self.Sphere.OnComponentEndOverlap`
  (params (OverlappedComponent :type "PrimitiveComponent Object Reference") (OtherActor :type "Actor Object Reference") (OtherComp :type "PrimitiveComponent Object Reference") (OtherBodyIndex :type Integer))
  (bind _asbp_3rd_pers (cast `/Game/TGJ/Sam/GP/3rdPers/BP/BP_3rdPers` OtherActor))
  (set `self.As BP Third Person Character` _asbp_3rd_pers)
  (remove `/Game/TGJ/Sam/GP/3rdPers/BP/GI_TGJ_Main.StartInteraction` (`self.As GI TGJ Main`) (delegate `Interaction`)))

(event `self.Sphere.OnComponentBeginOverlap`
  (params (OverlappedComponent :type "PrimitiveComponent Object Reference") (OtherActor :type "Actor Object Reference") (OtherComp :type "PrimitiveComponent Object Reference") (OtherBodyIndex :type Integer) (bFromSweep :type Boolean) (SweepResult :type "HitResult Structure (by ref)"))
  (bind _asbp_3rd_pers (cast `/Game/TGJ/Sam/GP/3rdPers/BP/BP_3rdPers` OtherActor))
  (set `self.As BP Third Person Character` _asbp_3rd_pers)
  (add `/Game/TGJ/Sam/GP/3rdPers/BP/GI_TGJ_Main.StartInteraction` (`self.As GI TGJ Main`) (delegate `Interaction`)))

(event `Interaction`
  (bind _as_gi_tgj_main (`self.As GI TGJ Main`))
  (`/Engine/EditorBlueprintResources/StandardMacros.DoOnce` false
    (:`Completed`
      (if (`self.UseGraduation`)
        (set `/Game/TGJ/Sam/GP/3rdPers/BP/GI_TGJ_Main.CurrentBPInt` self _as_gi_tgj_main)
        (`/Game/TGJ/Sam/GP/3rdPers/BP/GI_TGJ_Main.GradInteraction` _as_gi_tgj_main)
        (elif (`self.FX?`)
          (`self.InteractionFX`)
          (`KismetSystemLibrary.Delay` 0.25)
          (`self.InteractionEmote`)
          (else
            (`self.InteractionEmote`)))))))

(event `InteractionEmote`
  (bind _redtxt (`self.RedTXT`))
  (bind _bluetxt (`self.BlueTXT`))
  (bind _2emote_ (`self.2Emote?`))
  (bind _returnvalue (`|CreateWidget` "/Game/TGJ/Sam/UMG/W/W_S_InteractionEmote.W_S_InteractionEmote_C"))
  (if (`self.DetectChara?`)
    (if (`/Game/TGJ/Sam/GP/3rdPers/BP/BP_3rdPers.Blue?` (`self.As BP Third Person Character`))
      (if _2emote_ :!label _label
        (`/Game/TGJ/Sam/UMG/W/W_S_InteractionEmote.AnimRedBlue` _returnvalue _redtxt _bluetxt)
        (else
          (`/Game/TGJ/Sam/UMG/W/W_S_InteractionEmote.AnimRed` _returnvalue _redtxt)))
      (`UserWidget.AddToViewport` _returnvalue 0)
      (else
        (if _2emote_ :!label _label_2
          (`/Game/TGJ/Sam/UMG/W/W_S_InteractionEmote.AnimBlueRed` _returnvalue _bluetxt _redtxt)
          (else
            (`/Game/TGJ/Sam/UMG/W/W_S_InteractionEmote.AnimBlue` _returnvalue _bluetxt)))
        (`UserWidget.AddToViewport` _returnvalue 0)))
    (elif (`self.Blue?`)
      (goto _label_2)
      (else
        (goto _label)))))

(event `InteractionFX`
  (bind _niagara (`self.Niagara`))
  (bind _mesh (`self.Mesh`))
  (if (`/Game/TGJ/Sam/GP/3rdPers/BP/BP_3rdPers.Blue?` (`self.As BP Third Person Character`))
    (`NiagaraComponent.SetAsset` _niagara "/Game/TGJ/Sam/FX/NS/NS_S_B_QuickPaint.NS_S_B_QuickPaint" true)
    (`ActorComponent.Activate` _niagara false)
    (`PrimitiveComponent.CreateDynamicMaterialInstance` _mesh 0 "/Game/TGJ/Sam/Chara/Blue/M/M_SimpleColor.M_SimpleColor" "None")
    (else
      (`NiagaraComponent.SetAsset` _niagara "/Game/TGJ/Sam/FX/NS/NS_S_R_QuickPic.NS_S_R_QuickPic" true)
      (`ActorComponent.Activate` _niagara false)
      (`PrimitiveComponent.CreateDynamicMaterialInstance` _mesh 0 "/Game/TGJ/Sam/Chara/Rouge/M/Mi_SimpleColor.Mi_SimpleColor" "None"))))

(fn `UserConstructionScript`)