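; Environment spline tool that tiles static meshes along a spline in the construction script.
; It splits the spline into fixed-length sections and adds one deformed spline mesh component per section, with configurable collision.
; An optional variation mode picks among three meshes using a seeded random stream over an array, otherwise the first mesh is used.
; Tangents are clamped to section length, and a Fitting offset shifts each section's end point along the spline.
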(fn `Get End Position/Tangent`
  (params (Index :type Integer))
  (returns (Position :type "Vector Structure") (Tangent :type "Vector Structure"))
  (bind _spline (`self.Spline`))
  (bind _sectionlength (`self.SectionLength`))
  (bind _returnvalue (+ (* (+ Index 1) _sectionlength) (`self.Fitting`)))
  (return (`SplineComponent.GetLocationAtDistanceAlongSpline` _spline _returnvalue "Local") (`KismetMathLibrary.ClampVectorSize` (`SplineComponent.GetTangentAtDistanceAlongSpline` _spline _returnvalue "Local") 0.0 _sectionlength)))

(fn `Get Start Position/Tangent`
  (params (Index :type Integer))
  (returns (Position :type "Vector Structure") (Tangent :type "Vector Structure"))
  (bind _spline (`self.Spline`))
  (bind _sectionlength (`self.SectionLength`))
  (bind _returnvalue (* Index _sectionlength))
  (return (`SplineComponent.GetLocationAtDistanceAlongSpline` _spline _returnvalue "Local") (`KismetMathLibrary.ClampVectorSize` (`SplineComponent.GetTangentAtDistanceAlongSpline` _spline _returnvalue "Local") 0.0 _sectionlength)))

(fn `UserConstructionScript`
  (bind _loopindex (`self.LoopIndex`))
  (for _index (range (`KismetMathLibrary.FTrunc` (/ (`SplineComponent.GetSplineLength` (`self.Spline`)) (`self.SectionLength`))))
    (set `self.LoopIndex` _index)
    (bind _returnvalue (`AddComponent|NODE_AddSplineMeshComponent-0`))
    (if (`self.VariationOrNot`)
      (switch `string` (`KismetArrayLibrary.Array_RandomFromStream` (`self.Target Array`) (`self.Seed`))
        (:`Default`
          (`StaticMeshComponent.SetStaticMesh` _returnvalue (`self.Mesh1`) :!label _label))
        (:`1`
          (goto _label))
        (:`2`
          (`StaticMeshComponent.SetStaticMesh` _returnvalue (`self.Mesh2`)))
        (:`3`
          (`StaticMeshComponent.SetStaticMesh` _returnvalue (`self.Mesh3`))))
      (else
        (goto _label)))
    (`SplineMeshComponent.SetForwardAxis` _returnvalue "X" true)
    (bind (_position _tangent) (`self.Get Start Position/Tangent` _loopindex))
    (bind (_position_2 _tangent_2) (`self.Get End Position/Tangent` _loopindex))
    (`SplineMeshComponent.SetStartAndEnd` _returnvalue _position _tangent _position_2 _tangent_2 true)
    (`PrimitiveComponent.SetCollisionEnabled` _returnvalue (`self.MeshCollision`))))